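; BP_Bomb is a Bomberman bomb actor that explodes on a short fuse and kills nearby characters.
; The authority starts a timer on BeginPlay, which calls ShowExplosion and Explode.
; Explode destroys BombermanCharacter pawns found by a sphere overlap, destroys the bomb and re-enables bomb spawning on its BombOwner.
; ShowExplosion spawns an emitter only on the Remote branch of its authority switch.
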(event `self.ReceiveBeginPlay`
  (`/Engine/EditorBlueprintResources/ActorMacros.Switch Has Authority`
    (:`Authority`
      (`KismetSystemLibrary.K2_SetTimerDelegate` (delegate `OnExplode`) 2.0)
      (`KismetSystemLibrary.PrintString` "end timer" true true (struct :`R` 0.119838 :`B` 1.0 :`A` 1.0)))))

(event `OnExplode`
  (`self.ShowExplosion`)
  (`self.Explode`))

(event `Explode`
  (bind _bombowner (`self.BombOwner`))
  (`KismetSystemLibrary.PrintString` "hi dear")
  (bind _outactors (`KismetSystemLibrary.SphereOverlapActors` (`self.K2_GetActorLocation`) 200.0 (`|MakeArray` "ObjectTypeQuery3" :!type "EObjectTypeQuery Enum") "/Script/Bomberman.BombermanCharacter"))
  (for _array_element _outactors
    (`self.K2_DestroyActor` _array_element))
  (`self.K2_DestroyActor`)
  (`/Engine/EditorBlueprintResources/StandardMacros.IsValid` _bombowner
    (:`Is Valid`
      (set `/Game/Bomberman/Character/BP_BombermanCharacter.bCanSpawnBomb` true _bombowner))))

(event `ShowExplosion`
  (`/Engine/EditorBlueprintResources/ActorMacros.Switch Has Authority`
    (:`Remote`
      (`GameplayStatics.SpawnEmitterAtLocation` null (`self.K2_GetActorLocation`)))))

(fn `UserConstructionScript`)